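; Bernard Blueprint that fakes a walking animation by tilting its SceneRot component with Timelines.
; Each Tick compares the ManuallyWalking flag with the current animation state to start or stop the motion.
; While walking, a self-restarting Timeline drives a slight pitch sway.
; On stopping, a second Timeline eases pitch back to zero from an angle captured at that moment, and is cut short if walking resumes.
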(event `self.ReceiveTick`
  (params (DeltaSeconds :type "Float (single-precision)"))
  (`self.UpdateWalkingAnimation`))

(event `RestartWalkingAnimation`
  (bind (_direction _newtrack_0) (`Timeline|Timeline_0` :!via `PlayFromStart` :!label _label)
    (:`Update`
      (if (`self.isPlayingWalkingAnimation`)
        (`SceneComponent.K2_SetRelativeRotation` (`self.SceneRot`) (`KismetMathLibrary.MakeRotator` 90.0 (`KismetMathLibrary.Lerp` 0.0 1.5 _newtrack_0)) false false)))
    (:`Finished`
      (`self.RestartWalkingAnimation`))))

(event `UpdateWalkingAnimation`
  (if (`self.ManuallyWalking`)
    (if (not (`self.isPlayingWalkingAnimation`))
      (set `self.isPlayingWalkingAnimation` true)
      (if (`self.isPlayingStop`)
        (`|ExecutionSequence`
          (:`then_0`
            (set `self.isPlayingStop` false)
            (bind (_direction _newtrack_0) (`Timeline|Timeline_1` :!via `Stop` :!label _label_2)
              (:`Update`
                (`SceneComponent.K2_SetRelativeRotation` (`self.SceneRot`) (`KismetMathLibrary.MakeRotator` 90.0 (`KismetMathLibrary.Lerp` (`self.MeshRotationAngleToStopWalkingAnimation`) 0.0 _newtrack_0)) false false))
              (:`Finished`
                (set `self.isPlayingStop` false))))
          (:`then_1`
            (goto _label :!via `PlayFromStart`)))
        (else
          (goto _label :!via `PlayFromStart`))))
    (elif (`self.isPlayingWalkingAnimation`)
      (set `self.isPlayingWalkingAnimation` false)
      (`|ExecutionSequence`
        (:`then_0`
          (goto _label :!via `Stop`))
        (:`then_1`
          (set `self.MeshRotationAngleToStopWalkingAnimation` (.pitch (`SceneComponent.RelativeRotation` (`self.Scene`))))
          (set `self.isPlayingStop` true)
          (goto _label_2 :!via `PlayFromStart`))))))

(fn `UserConstructionScript`)