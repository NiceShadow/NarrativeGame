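; BP_FoldTest is an actor for Room 1 that plays an opening animation on a book and room pieces, apparently a fold-out test.
; Open slows the actor's custom time dilation, plays a sound and starts one-shot animations on the book, ground, carpets, and safe and unsafe elements.
; SetRightWallTransparent swaps the safe elements' first material between right-wall and alpha versions, mirroring the state to MainCharacter's R1RightwallTransparent flag.
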(event `Open`
  (set `self.CustomTimeDilation` 0.605)
  (`GameplayStatics.PlaySound2D` null 1.0 1.0 0.0 null null)
  (`SkeletalMeshComponent.PlayAnimation` (`self.safeE`) "/Game/Lewin/Room1_AnimatedMesh/safeElements/safElementse_Anim.safElementse_Anim" false)
  (`SkeletalMeshComponent.PlayAnimation` (`self.book`) "/Game/Jana/bookwUV/bookUV_17_Anim.bookUV_17_Anim" false)
  (`SkeletalMeshComponent.PlayAnimation` (`self.ground`) "/Game/Lewin/Room1_AnimatedMesh/floor/room1_ground_Anim.room1_ground_Anim" false)
  (`SkeletalMeshComponent.PlayAnimation` (`self.UnSafe`) "/Game/Jana/room1_UNsafeelements_Anim.room1_UNsafeelements_Anim" false)
  (`SkeletalMeshComponent.PlayAnimation` (`self.carpets`) "/Game/Jana/room1_allcarpets_Anim.room1_allcarpets_Anim" false))

(event `SetRightWallTransparent`
  (params (yes :type Boolean))
  (bind _returnvalue (`GameplayStatics.GetPlayerCharacter` 0))
  (bind _safee (`self.safeE`))
  (if yes
    (`PrimitiveComponent.SetMaterial` _safee 0 "/Game/Materials/Assets/Room1/Textures/RightWallAlpha.RightWallAlpha")
    (bind _asmain_character (cast `/Game/Lewin/Blueprints/MainCharacter` _returnvalue))
    (set `/Game/Lewin/Blueprints/MainCharacter.r1_rightwallTransparent` true _asmain_character)
    (else
      (`PrimitiveComponent.SetMaterial` _safee 0 "/Game/Materials/Assets/Room1/Textures/M_r1_right_wall.M_r1_right_wall")
      (bind _asmain_character_2 (cast `/Game/Lewin/Blueprints/MainCharacter` _returnvalue))
      (set `/Game/Lewin/Blueprints/MainCharacter.r1_rightwallTransparent` false _asmain_character_2))))

(fn `UserConstructionScript`)