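; Player controller that runs pausing, music, audio and graphics settings, and inventory drag targeting.
; On BeginPlay it generates a random four-digit safe PIN, starts menu music and applies saved volume and quality settings through audio components and console commands, toggling Niagara actors by quality.
; While dragging, it traces from the camera through the cursor and highlights the item when the hit actor's "drop" tag ID matches, subject to special-case puzzle checks.
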(event `Key|Escape` :paused true
  (params (Key :type "Key Structure"))
  ;[1 1 1] Pause/Unpause PC
  (:`Pressed`
    (if (`self.Can PauseGame`) :!label _label
      (`self.PauseGame` (not (`GameplayStatics.IsGamePaused`)))
      (bind _asmain_character (cast `/Game/Lewin/Blueprints/MainCharacter` (`GameplayStatics.GetPlayerCharacter` 0)))
      (`/Game/Blueprints/WB_NormalCursor.Interact` (`/Game/Lewin/Blueprints/MainCharacter.CustomCursor` _asmain_character) false 0))))

(event `SetGrapchis`
  (params (GR :type Integer))
  (bind _returnvalue (`GameplayStatics.GetPlayerController` 0))
  (bind _returnvalue_2 (`GameplayStatics.GetPlayerController` 0))
  (bind _returnvalue_3 (`GameplayStatics.GetPlayerController` 0))
  (bind _output_get (set `self.GR` GR))
  (switch `int` _output_get
    (:`0`
      (`KismetSystemLibrary.ExecuteConsoleCommand` "sg.TextureQuality 0" _returnvalue_3)
      (`KismetSystemLibrary.ExecuteConsoleCommand` "sg.EffectsQuality 0" _returnvalue_3)
      (`KismetSystemLibrary.ExecuteConsoleCommand` "r.ViewDistanceScale 0" _returnvalue_3)
      (`KismetSystemLibrary.ExecuteConsoleCommand` "sg.ShadowQuality 0" null)
      (`KismetSystemLibrary.ExecuteConsoleCommand` "r.ScreenPercentage 60" null)
      (bind _outactors (`GameplayStatics.GetAllActorsOfClass` "/Script/Niagara.NiagaraActor"))
      (for _array_element _outactors
        (`ActorComponent.Deactivate` (`NiagaraActor.NiagaraComponent` _array_element))))
    (:`1`
      (`KismetSystemLibrary.ExecuteConsoleCommand` "sg.TextureQuality 2" _returnvalue_2)
      (`KismetSystemLibrary.ExecuteConsoleCommand` "sg.EffectsQuality 2" _returnvalue_2)
      (`KismetSystemLibrary.ExecuteConsoleCommand` "r.ViewDistanceScale 0.5" _returnvalue_2)
      (`KismetSystemLibrary.ExecuteConsoleCommand` "sg.ShadowQuality 2" null)
      (`KismetSystemLibrary.ExecuteConsoleCommand` "r.ScreenPercentage 90" null)
      (bind _outactors_2 (`GameplayStatics.GetAllActorsOfClass` "/Script/Niagara.NiagaraActor"))
      (for _array_element_2 _outactors_2
        (`ActorComponent.Deactivate` (`NiagaraActor.NiagaraComponent` _array_element_2))))
    (:`2`
      (`KismetSystemLibrary.ExecuteConsoleCommand` "sg.TextureQuality 3" _returnvalue)
      (`KismetSystemLibrary.ExecuteConsoleCommand` "sg.EffectsQuality 3" _returnvalue)
      (`KismetSystemLibrary.ExecuteConsoleCommand` "r.ViewDistanceScale 1" _returnvalue)
      (`KismetSystemLibrary.ExecuteConsoleCommand` "sg.ShadowQuality 3" null)
      (`KismetSystemLibrary.ExecuteConsoleCommand` "r.ScreenPercentage 100" null)
      (bind _outactors_3 (`GameplayStatics.GetAllActorsOfClass` "/Script/Niagara.NiagaraActor"))
      (for _array_element_3 _outactors_3
        (`ActorComponent.Activate` (`NiagaraActor.NiagaraComponent` _array_element_3) false)))))

(event `Key|P` :paused true
  (params (Key :type "Key Structure"))
  ;[1 1 1] Pause/Unpause PC
  (:`Pressed`
    (goto _label)))

(event `StartMusicMenu`
  (`/Engine/EditorBlueprintResources/StandardMacros.IsValid` (`self.MenuSoundPC`)
    (:`Is Not Valid`
      (bind _returnvalue (`GameplayStatics.SpawnSound2D` "/Game/Sounds/SFX/Three_Pages.Three_Pages" (`self.MusicVolume`) 1.0 0.0 null false false))
      (set `self.MenuSoundPC` _returnvalue))))

(event `self.ReceiveBeginPlay`
  (set `self.bShowMouseCursor` true)
  (`self.CreateSafePin`)
  (`self.StartMusicMenu`)
  (`KismetSystemLibrary.PrintString` (`self.SafePIN`))
  (bind _returnvalue (`GameplayStatics.LoadGameFromSlot` "sg"))
  (bind _asour_save_game (cast `/Game/Lewin/OurSaveGame` _returnvalue))
  (set `self.MusicVolume` (`/Game/Lewin/OurSaveGame.s_m` _asour_save_game))
  (set `self.SoundEffectsVolume` (`/Game/Lewin/OurSaveGame.s_fx` _asour_save_game))
  (set `self.VoiceVolume` (`/Game/Lewin/OurSaveGame.s_v` _asour_save_game))
  (set `self.GR` (`/Game/Lewin/OurSaveGame.gr` _asour_save_game))
  (`self.UpdateVolumeFX` (`self.SoundEffectsVolume`))
  (`self.UpdateVolume_m` (`self.MusicVolume`))
  (`self.UpdateVolume_v` (`self.VoiceVolume`))
  (`self.SetGrapchis` (`self.GR`)))

(event `StartGamePlaySound`
  (`/Engine/EditorBlueprintResources/StandardMacros.IsValid` (`self.GameplaySoundPC`)
    (:`Is Not Valid`
      (`AudioComponent.FadeOut` (`self.MenuSoundPC`) 2.0 0.0 "Linear")
      (bind _returnvalue (`GameplayStatics.SpawnSound2D` "/Game/Sounds/SFX/00_-_Desktop_-_Highly_unfunctional_Hotel_Room2.00_-_Desktop_-_Highly_unfunctional_Hotel_Room2" (`self.MusicVolume`) 1.0 0.0 null false false))
      (set `self.GameplaySoundPC` _returnvalue))))

(event `UpdateVolumeFX`
  (params (VoiceVolume :type "Float (double-precision)"))
  (set `self.SoundEffectsVolume` (`KismetMathLibrary.FClamp` VoiceVolume 0.01 5.0)))

(event `SetupRefs`
  (bind _asbp_our_hud (cast `/Game/Blueprints/BP_OurHUD` (`self.GetHUD`)))
  (bind _output_get (set `self.GameUIRef` (`/Game/Blueprints/BP_OurHUD.GameUI` _asbp_our_hud)))
  (set `self.InventoryRef` (`/Game/Lewin/UI/WB_GameUI.WB_Inventory` _output_get))
  (set `self.DiaRef` (`/Game/Blueprints/BP_OurHUD.DialogueWindow` _asbp_our_hud))
  (set `self.MenuRef` (`/Game/Blueprints/BP_OurHUD.MenuRef` _asbp_our_hud)))

(event `UpdateVolume_v`
  (params (VoiceVolume :type "Float (double-precision)"))
  (bind _diaref (`self.DiaRef`))
  (bind _currentsound (`/Game/Daniel/Blueprints/BP_DialogueWindow.CurrentSound` _diaref))
  (set `self.VoiceVolume` (`KismetMathLibrary.FClamp` VoiceVolume 0.01 5.0))
  (`/Engine/EditorBlueprintResources/StandardMacros.IsValid` _diaref
    (:`Is Valid`
      (`/Engine/EditorBlueprintResources/StandardMacros.IsValid` _currentsound
        (:`Is Valid`
          (`AudioComponent.AdjustVolume` _currentsound 0.0 (`self.VoiceVolume`) "Linear"))))))

(event `PauseGame`
  (params (Pause :type Boolean))
  (`/Game/Daniel/Blueprints/BP_DialogueWindow.Pause` (`self.DiaRef`) Pause)
  (if Pause
    (`GameplayStatics.SetGamePaused` true)
    (if (`GameplayStatics.IsGamePaused`) :!label _label_2
      (bind _asbp_our_hud (cast `/Game/Blueprints/BP_OurHUD` (`self.GetHUD` (`GameplayStatics.GetPlayerController` 0))))
      (`/Game/Lewin/UI/WB_PauseMenu.Show` (`/Game/Lewin/UI/WB_GameUI.WB_PauseMenu` (`/Game/Blueprints/BP_OurHUD.GameUI` _asbp_our_hud)) true)
      (else
        (bind _asbp_our_hud_2 (cast `/Game/Blueprints/BP_OurHUD` (`self.GetHUD` (`GameplayStatics.GetPlayerController` 0))))
        (`/Game/Lewin/UI/WB_PauseMenu.Show` (`/Game/Lewin/UI/WB_GameUI.WB_PauseMenu` (`/Game/Blueprints/BP_OurHUD.GameUI` _asbp_our_hud_2)) false)))
    (else
      (bind _asbp_our_hud_3 (cast `/Game/Blueprints/BP_OurHUD` (`self.GetHUD` (`GameplayStatics.GetPlayerController` 0))))
      (if (`/Game/Lewin/UI/WB_PauseMenu.InMainPause?` (`/Game/Lewin/UI/WB_GameUI.WB_PauseMenu` (`/Game/Blueprints/BP_OurHUD.GameUI` _asbp_our_hud_3)))
        (`GameplayStatics.SetGamePaused` false)
        (goto _label_2)))))

(event `UpdateVolume_m`
  (params (MusicVolume :type "Float (double-precision)"))
  (bind _gameplaysoundpc (`self.GameplaySoundPC`))
  (bind _menusoundpc (`self.MenuSoundPC`))
  (set `self.MusicVolume` (`KismetMathLibrary.FClamp` MusicVolume 0.01 5.0))
  (`|ExecutionSequence`
    (:`then_0`
      (`/Engine/EditorBlueprintResources/StandardMacros.IsValid` _menusoundpc
        (:`Is Valid`
          (`AudioComponent.AdjustVolume` _menusoundpc 0.0 (`self.MusicVolume`) "Linear"))))
    (:`then_1`
      (`/Engine/EditorBlueprintResources/StandardMacros.IsValid` _gameplaysoundpc
        (:`Is Valid`
          (`AudioComponent.AdjustVolume` _gameplaysoundpc 0.0 (`self.MusicVolume`) "Linear"))))))

(event `GetCursorFromDrag`
  (params (Cursor :type "Vector2D Structure"))
  (bind _returnvalue (`self.K2_GetActorLocation` (`GameplayStatics.GetPlayerCameraManager` 0)))
  (bind ((`ID_2_B0C2F0A14A73D287B352E4A900FEEFD1` _id)) (break `/Game/Lewin/item_Structure` (`/Game/Lewin/UI/WB_ItemDrag.ItemData` (`/Game/Lewin/UI/WB_Inventory.CurrentDragOP` (`self.InventoryRef`)))))
  (if (`self.CanInteract`)
    (bind _returnvalue_2 (`WidgetLayoutLibrary.GetPlayerScreenWidgetGeometry` self))
    (bind (_outhit _returnvalue_3) (`KismetSystemLibrary.LineTraceSingle` _returnvalue (+ _returnvalue (* (`.WorldDirection` (`GameplayStatics.DeprojectScreenToWorld` self (* (`SlateBlueprintLibrary.AbsoluteToLocal` _returnvalue_2 Cursor) (`WidgetLayoutLibrary.GetViewportScale`)))) 2000.0)) "TraceTypeQuery1"))
    (if _returnvalue_3
      (set `self.HitResults` true)
      (bind (_bblockinghit _binitialoverlap _time _distance _location _impactpoint _normal _impactnormal _physmat _hitactor) (`GameplayStatics.BreakHitResult` _outhit))
      (if (!= _hitactor (`self.HitActorBefore`))
        (set `self.HitActorBefore` _hitactor)
        (bind _tags (`Actor.Tags` _hitactor))
        (bind _returnvalue_4 (`KismetArrayLibrary.Array_Length` _tags))
        (if (> _returnvalue_4 0)
          (bind _returnvalue_5 (`KismetStringLibrary.Conv_NameToString` (`|GetArrayItem` _tags)))
          (if (`KismetStringLibrary.Contains` _returnvalue_5 "drop")
            (if (== (`KismetStringLibrary.Conv_StringToInt` (`KismetStringLibrary.GetSubstring` _returnvalue_5 5 (- (`KismetStringLibrary.Len` _returnvalue_5) 5))) _id)
              (bind _isallowed (`self.SpecialCasesHover` _id :!label _label_3))
              (if _isallowed
                (set `self.isHighlighted` true)
                (`/Game/Lewin/UI/WB_ItemDrag.Highlight` (`/Game/Lewin/UI/WB_Inventory.CurrentDragOP` (`self.InventoryRef`)) true false))
              (elif (> _returnvalue_4 1)
                (bind _returnvalue_6 (`KismetStringLibrary.Conv_NameToString` (`|GetArrayItem` _tags 1)))
                (if (== _id (`KismetStringLibrary.Conv_StringToInt` (`KismetStringLibrary.GetSubstring` _returnvalue_6 5 (- (`KismetStringLibrary.Len` _returnvalue_6) 5))))
                  (goto _label_3)))))
          (else
            (if (`self.isHighlighted`) :!label _label_4
              (`/Game/Lewin/UI/WB_ItemDrag.Highlight` (`/Game/Lewin/UI/WB_Inventory.CurrentDragOP` (`self.InventoryRef`)) false false)
              (set `self.isHighlighted` false)))))
      (elif (`self.HitResults`)
        (set `self.HitActorBefore` null)
        (`/Game/Lewin/UI/WB_ItemDrag.Highlight` (`/Game/Lewin/UI/WB_Inventory.CurrentDragOP` (`self.InventoryRef`)) false false)
        (set `self.HitResults` false)))
    (else
      (goto _label_4))))

(fn `CreateSafePin`
  (set `self.SafePIN` (`KismetStringLibrary.Concat_StrStr` (`self.SafePIN`) (`KismetStringLibrary.Conv_IntToString` (`KismetMathLibrary.RandomIntegerInRange` 0 9))))
  (set `self.SafePIN` (`KismetStringLibrary.Concat_StrStr` (`self.SafePIN`) (`KismetStringLibrary.Conv_IntToString` (`KismetMathLibrary.RandomIntegerInRange` 0 9))))
  (set `self.SafePIN` (`KismetStringLibrary.Concat_StrStr` (`self.SafePIN`) (`KismetStringLibrary.Conv_IntToString` (`KismetMathLibrary.RandomIntegerInRange` 0 9))))
  (set `self.SafePIN` (`KismetStringLibrary.Concat_StrStr` (`self.SafePIN`) (`KismetStringLibrary.Conv_IntToString` (`KismetMathLibrary.RandomIntegerInRange` 0 9)))))

(fn `SpecialCasesHover`
  (params (ID :type Integer))
  (returns (isAllowed :type Boolean))
  (if (or (== ID 2) (== ID 4))
    (if (`/Game/Lewin/Blueprints/BP_FoldTest.r1_carpetTVmoved` (`self.BookRef`))
      (return true))
    (else
      (return true))))

(fn `UserConstructionScript`)