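; Character component that routes the player's interaction with room objects to the matching dialogue in the HUD's dialogue window.
; Interact switches on a Selection value covering furniture, props and doors, plus the washers and dryers of a second room, calling one dialogue function each; two dryers share the empty response.
; A helper fetches the DialogueWindow by casting the first player controller's HUD to BP_OurHUD.
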(event `Interact`
  (params (Selection :type String))
  (bind _newparam (`self.GetDialogueW`))
  (bind _newparam_2 (`self.GetDialogueW`))
  (switch `string` Selection
    (:`tv`
      (`/Game/Daniel/Blueprints/BP_DialogueWindow.Interact_TV` _newparam))
    (:`shelf`
      (`/Game/Daniel/Blueprints/BP_DialogueWindow.Interact_Shelf` _newparam))
    (:`mirror`
      (`/Game/Daniel/Blueprints/BP_DialogueWindow.Interact_Mirror` _newparam))
    (:`bed`
      (`/Game/Daniel/Blueprints/BP_DialogueWindow.Interact Bed` _newparam))
    (:`couch`
      (`/Game/Daniel/Blueprints/BP_DialogueWindow.Interact Couch` _newparam))
    (:`notepad`
      (`/Game/Daniel/Blueprints/BP_DialogueWindow.Notepad Found` _newparam))
    (:`safe`
      (`/Game/Daniel/Blueprints/BP_DialogueWindow.Interact Safe` _newparam))
    (:`carpet`
      (`/Game/Daniel/Blueprints/BP_DialogueWindow.Interact Carpet` _newparam))
    (:`phone`
      (`/Game/Daniel/Blueprints/BP_DialogueWindow.Interact Phone` _newparam))
    (:`bdoor`
      (`/Game/Daniel/Blueprints/BP_DialogueWindow.Interact Bdoor` _newparam))
    (:`door`
      (`/Game/Daniel/Blueprints/BP_DialogueWindow.Interact Door` _newparam))
    (:`chute`
      (`/Game/Daniel/Blueprints/BP_DialogueWindow.Interact LaundryChute` _newparam))
    (:`dials`
      (`/Game/Daniel/Blueprints/BP_DialogueWindow.InteractLeftDesk` _newparam))
    (:`sharpener`
      (`/Game/Daniel/Blueprints/BP_DialogueWindow.InteractRightDesk` _newparam))
    (:`window`
      (`/Game/Daniel/Blueprints/BP_DialogueWindow.Interact Window` _newparam))
    (:`nail`
      (`/Game/Daniel/Blueprints/BP_DialogueWindow.Interact Plant` _newparam))
    (:`wmachine`
      (`/Game/Daniel/Blueprints/BP_DialogueWindow.Interact wmachine` _newparam_2))
    (:`kdoor`
      (`/Game/Daniel/Blueprints/BP_DialogueWindow.Room2 Door` _newparam_2))
    (:`wmachine1`
      (`/Game/Daniel/Blueprints/BP_DialogueWindow.Room2 Wmachine1` _newparam_2))
    (:`wmachine2`
      (`/Game/Daniel/Blueprints/BP_DialogueWindow.Room2 Wmachine2` _newparam_2))
    (:`wmachine3`
      (`/Game/Daniel/Blueprints/BP_DialogueWindow.Room2 Wmachine3` _newparam_2))
    (:`dryer1`
      (`/Game/Daniel/Blueprints/BP_DialogueWindow.Room2 Dryer Empty` _newparam_2 :!label _label))
    (:`dryer2`
      (goto _label))
    (:`dryer3`
      (`/Game/Daniel/Blueprints/BP_DialogueWindow.Room2 Dryer TooS` _newparam_2))))

(fn `GetDialogueW`
  (returns (NewParam :type "/Game/Daniel/Blueprints/BP_DialogueWindow Object Reference"))
  (bind _asbp_our_hud (cast `/Game/Blueprints/BP_OurHUD` (`PlayerController.GetHUD` (`GameplayStatics.GetPlayerController` 0))))
  (return (`/Game/Blueprints/BP_OurHUD.DialogueWindow` _asbp_our_hud)))